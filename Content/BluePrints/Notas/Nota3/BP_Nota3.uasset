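; BP_Nota3 is the third collectible note, shown as a UI widget while an actor overlaps its collision.
; The first overlap passes a DoOnce and increments NotasObtenidas on BP_FirstPersonCharacter.
; Every begin overlap plays a sound and creates Widget_Nota3; end overlap replays the sound and calls the widget's fade-out.
; An all-notes-collected message check exists but is disconnected, so it never runs.
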(event `self.CollisionNota3.OnComponentBeginOverlap`
  (params (OverlappedComponent :type "PrimitiveComponent Object Reference") (OtherActor :type "Actor Object Reference") (OtherComp :type "PrimitiveComponent Object Reference") (OtherBodyIndex :type Integer) (bFromSweep :type Boolean) (SweepResult :type "HitResult Structure (by ref)"))
  ;[1 1 1] Mostrar/Ocultar nota
  (`|ExecutionSequence`
    (:`then_0`
      ;[1 1 1] Agregar +1 nota al contador
      (`/Engine/EditorBlueprintResources/StandardMacros.DoOnce` false
        (:`Completed`
          (bind _asbp_first_person_character (cast `/Game/FirstPerson/Blueprints/BP_FirstPersonCharacter` OtherActor))
          (set `/Game/FirstPerson/Blueprints/BP_FirstPersonCharacter.NotasObtenidas` (+ (`/Game/FirstPerson/Blueprints/BP_FirstPersonCharacter.NotasObtenidas` _asbp_first_person_character) 1) _asbp_first_person_character))))
    (:`then_1`
      (`GameplayStatics.PlaySoundAtLocation` "/Game/BluePrints/Notas/NotasDejar.NotasDejar" (`self.K2_GetActorLocation` OtherActor) (struct) 1.0 1.0 0.0 null null null null)
      (bind _returnvalue (`|CreateWidget` "/Game/BluePrints/Notas/Nota3/Widget_Nota3.Widget_Nota3_C"))
      (`UserWidget.AddToViewport` _returnvalue 0))))

(event `self.CollisionNota3.OnComponentEndOverlap`
  (params (OverlappedComponent :type "PrimitiveComponent Object Reference") (OtherActor :type "Actor Object Reference") (OtherComp :type "PrimitiveComponent Object Reference") (OtherBodyIndex :type Integer))
  ;[1 1 1] Mostrar/Ocultar nota
  (`GameplayStatics.PlaySoundAtLocation` "/Game/BluePrints/Notas/NotasDejar.NotasDejar" (`self.K2_GetActorLocation` OtherActor) (struct) 1.0 1.0 0.0 null null null null)
  (`/Game/BluePrints/Notas/Nota3/Widget_Nota3.Fade out3` (stale `self.CollisionNota3.OnComponentBeginOverlap` _returnvalue)))

(fn `UserConstructionScript`)