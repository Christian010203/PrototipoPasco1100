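; Door actor that opens with the E key only when the first-person character holds the third key (TengoLlave3).
; Overlapping its collision plays a padlock sound and shows an interaction widget, enabling input for the player character; leaving disables input and fades the widget.
; With the key, E destroys the collision, plays a door sound and swings the door's yaw through a timeline; otherwise it shows no-key feedback with a metallic sound.
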(event `Key|E`
  (params (Key :type "Key Structure"))
  (:`Pressed`
    (if (`/Game/FirstPerson/Blueprints/BP_FirstPersonCharacter.TengoLlave3` (stale `self.CollisionPuerta3.OnComponentBeginOverlap` _asbp_first_person_character))
      (`ActorComponent.K2_DestroyComponent` (`self.CollisionPuerta3`))
      (`GameplayStatics.PlaySound2D` "/Game/Sonidos/021_Puerta_4.021_Puerta_4" 1.0 1.0 0.0 null null)
      (bind (_direction _newtrack_0) (`Timeline|Timeline`)
        (:`Update`
          (`SceneComponent.K2_SetRelativeRotation` (`self.Puerta3`) (`KismetMathLibrary.MakeRotator` 0.0 0.0 (* _newtrack_0 -20.0)) false false)))
      (else
        (`/Game/Widgets/Llaves/Widget_Interactuar.NoLlave` (stale `self.CollisionPuerta3.OnComponentBeginOverlap` _returnvalue))
        (`GameplayStatics.PlaySoundAtLocation` "/Game/Sonidos/002_Ambiente_metalico_1.002_Ambiente_metalico_1" (`self.K2_GetActorLocation`) (struct) 1.0 1.0 0.0 null null null null)))))

(event `self.CollisionPuerta3.OnComponentBeginOverlap`
  (params (OverlappedComponent :type "PrimitiveComponent Object Reference") (OtherActor :type "Actor Object Reference") (OtherComp :type "PrimitiveComponent Object Reference") (OtherBodyIndex :type Integer) (bFromSweep :type Boolean) (SweepResult :type "HitResult Structure (by ref)"))
  (`|ExecutionSequence`
    (:`then_0`
      (`GameplayStatics.PlaySoundAtLocation` "/Game/Sonidos/001_Abrir_Candados.001_Abrir_Candados" (`self.K2_GetActorLocation`) (struct) 1.0 1.0 0.0 null null null null)
      (bind _returnvalue (`|CreateWidget` "/Game/Widgets/Llaves/Widget_Interactuar.Widget_Interactuar_C"))
      (`UserWidget.AddToViewport` _returnvalue 0))
    (:`then_1`
      (bind _asbp_first_person_character (cast `/Game/FirstPerson/Blueprints/BP_FirstPersonCharacter` OtherActor))
      (`self.EnableInput` (`GameplayStatics.GetPlayerController` 0)))))

(event `self.CollisionPuerta3.OnComponentEndOverlap`
  (params (OverlappedComponent :type "PrimitiveComponent Object Reference") (OtherActor :type "Actor Object Reference") (OtherComp :type "PrimitiveComponent Object Reference") (OtherBodyIndex :type Integer))
  (`|ExecutionSequence`
    (:`then_0`
      (cast `/Game/FirstPerson/Blueprints/BP_FirstPersonCharacter` OtherActor)
      (`self.DisableInput` (`GameplayStatics.GetPlayerController` 0)))
    (:`then_1`
      (`/Game/Widgets/Llaves/Widget_Interactuar.Fade Out interactuarE` (stale `self.CollisionPuerta3.OnComponentBeginOverlap` _returnvalue)))))

(event `self.ReceiveBeginPlay`)

(fn `UserConstructionScript`)