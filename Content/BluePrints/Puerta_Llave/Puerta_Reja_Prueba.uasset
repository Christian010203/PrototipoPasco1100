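; Test Blueprint for a barred gate that the player opens and closes with the E key, provided they carry key 1.
; The collision box casts to BP_FirstPersonCharacter, stores it, and enables input only during overlap.
; If the character's TengoLlave1 flag is true, a FlipFlop alternately plays and reverses the Abrircerrar timeline, swinging Reja1 around its yaw axis.
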(event `Key|E`
  (params (Key :type "Key Structure"))
  (:`Pressed`
    (if (`/Game/FirstPerson/Blueprints/BP_FirstPersonCharacter.TengoLlave1` (stale `self.BoxColision.OnComponentBeginOverlap` _asbp_first_person_character))
      (`/Engine/EditorBlueprintResources/StandardMacros.FlipFlop`
        (:`A`
          (bind (_direction _newtrack_0) (`Timeline|Abrir/cerrar` :!label _label)
            (:`Update`
              (`SceneComponent.K2_SetRelativeRotation` (`self.Reja1`) (`KismetMathLibrary.MakeRotator` 0.0 0.0 (* _newtrack_0 -90.0)) false false))))
        (:`B`
          (goto _label :!via `Reverse`))))))

(event `self.BoxColision.OnComponentBeginOverlap`
  (params (OverlappedComponent :type "PrimitiveComponent Object Reference") (OtherActor :type "Actor Object Reference") (OtherComp :type "PrimitiveComponent Object Reference") (OtherBodyIndex :type Integer) (bFromSweep :type Boolean) (SweepResult :type "HitResult Structure (by ref)"))
  (bind _asbp_first_person_character (cast `/Game/FirstPerson/Blueprints/BP_FirstPersonCharacter` OtherActor))
  (`self.EnableInput` (`GameplayStatics.GetPlayerController` 0)))

(event `self.BoxColision.OnComponentEndOverlap`
  (params (OverlappedComponent :type "PrimitiveComponent Object Reference") (OtherActor :type "Actor Object Reference") (OtherComp :type "PrimitiveComponent Object Reference") (OtherBodyIndex :type Integer))
  (cast `/Game/FirstPerson/Blueprints/BP_FirstPersonCharacter` OtherActor)
  (`self.DisableInput` (`GameplayStatics.GetPlayerController` 0)))

(event `self.ReceiveBeginPlay`)

(fn `UserConstructionScript`)